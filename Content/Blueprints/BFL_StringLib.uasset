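; Blueprint function library that formats a duration in seconds as a zero-padded MM:SS.cc timer display.
; BFL_SecondsToTimeString floors out minutes, remaining seconds and hundredths, prefixes a "0" to single-digit values, and appends them with ":" and "." separators.
; BFL_FloatSecondsToTextTime wraps that string function and returns the result as Text.
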(fn `BFL_FloatSecondsToTextTime`
  (params (InSeconds :type "Float (double-precision)"))
  (returns (OutTime :type Text))
  (return (`KismetTextLibrary.Conv_StringToText` (`self.BFL_SecondsToTimeString` InSeconds))))

(fn `BFL_SecondsToTimeString`
  (params (InTimeSeconds :type "Float (double-precision)"))
  (returns (OutTimeString :type String))
  (bind _returnvalue (mod InTimeSeconds 60.0))
  (bind _returnvalue_2 (`KismetMathLibrary.FFloor` (/ InTimeSeconds 60.0)))
  (bind _returnvalue_3 (`KismetMathLibrary.FFloor` (mod InTimeSeconds 60.0)))
  (bind _returnvalue_4 (`KismetMathLibrary.FFloor` (* (- _returnvalue (`KismetMathLibrary.Conv_IntToDouble` (`KismetMathLibrary.FFloor` _returnvalue))) 100.0)))
  (return (`KismetStringLibrary.Concat_StrStr` (select `bool` (> _returnvalue_2 9) :`false` (`KismetStringLibrary.Concat_StrStr` "0" (`KismetStringLibrary.Conv_IntToString` _returnvalue_2)) :`true` (`KismetStringLibrary.Conv_IntToString` _returnvalue_2)) ":" (select `bool` (> _returnvalue_3 9) :`false` (`KismetStringLibrary.Concat_StrStr` "0" (`KismetStringLibrary.Conv_IntToString` _returnvalue_3)) :`true` (`KismetStringLibrary.Conv_IntToString` _returnvalue_3)) "." (select `bool` (> _returnvalue_4 9) :`false` (`KismetStringLibrary.Concat_StrStr` "0" (`KismetStringLibrary.Conv_IntToString` _returnvalue_4)) :`true` (`KismetStringLibrary.Conv_IntToString` _returnvalue_4)))))