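; Checkpoint actor for a driving course that detects when a VehicleBlueprint passes through it in the correct direction.
; When the vehicle leaves the Trigger, a dot product of its velocity and the Arrow's forward vector rejects wrong-way passes.
; A valid pass prints a debug message, fires OnCheckPointCleared with CheckpointNumber and hides the checkpoint.
; ShowCheckPoint and HideCheckPoint toggle the particle marker and the Trigger's overlap events together.
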(event `self.Trigger.OnComponentEndOverlap`
  (params (OverlappedComponent :type "PrimitiveComponent Object Reference") (OtherActor :type "Actor Object Reference") (OtherComp :type "PrimitiveComponent Object Reference") (OtherBodyIndex :type Integer))
  ;[1 1 1] 체크포인트에 도달했는지 체크
  (bind _asvehicle_blueprint (cast `/Game/VehicleAdvBP/Blueprints/VehicleBlueprint` OtherActor))
  (if (> (`KismetMathLibrary.Dot_VectorVector` (`self.GetVelocity` _asvehicle_blueprint) (`KismetMathLibrary.Conv_RotatorToVector` (`SceneComponent.K2_GetComponentRotation` (`self.Arrow`)))) 0.0)
    (`KismetSystemLibrary.PrintString` (`KismetStringLibrary.Concat_StrStr` (`KismetSystemLibrary.GetDisplayName` self) " Cleared!") true true (struct :`G` 0.66 :`B` 1.0 :`A` 1.0) 60.0)
    (`self.EventDispatcher_OnCheckPointCleared` (`self.CheckpointNumber`))
    (`self.HideCheckPoint`)))

(fn `HideCheckPoint`
  (`SceneComponent.SetHiddenInGame` (`self.ParticleSystem`) true false)
  (set `PrimitiveComponent.bGenerateOverlapEvents` false (`self.Trigger`)))

(fn `ShowCheckPoint`
  (`SceneComponent.SetHiddenInGame` (`self.ParticleSystem`) false false)
  (set `PrimitiveComponent.bGenerateOverlapEvents` true (`self.Trigger`)))

(fn `UserConstructionScript`)